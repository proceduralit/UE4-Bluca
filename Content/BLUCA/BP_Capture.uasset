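; Capture actor that paints hit marks on skeletal meshes into render-target masks that fade over time.
; PaintActor briefly swaps material slot 0 for an unwrap material fed the hit location, then triggers a scene capture; its BrushRadius input is overridden by a constant.
; Each tick draws the fade and buffer render targets, then clears the draw mask.
; Startup creates the dynamic materials and publishes capture size and location to MPC_Global.
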(event EventBeginPlay
  (Utilities|InitializeParameters
    (:Out
      (bind _returnvalue (Rendering|Material|CreateDynamicMaterialInstance "/Game/BLUCA/M_DrawOutput.M_DrawOutput" "None" "None" :!class /Script/Engine.KismetMaterialLibrary))
      (Variables|Default|SetUnwrapMaterial _returnvalue)
      (bind _returnvalue_2 (Rendering|Material|CreateDynamicMaterialInstance "/Game/BLUCA/M_DrawMaskBuffer.M_DrawMaskBuffer" "None" "None" :!class /Script/Engine.KismetMaterialLibrary))
      (Variables|Default|SetBufferMaterial _returnvalue_2)
      (Rendering|ClearRenderTarget2D "/Game/BLUCA/RT_DrawMaskBuffer.RT_DrawMaskBuffer")
      (bind _returnvalue_3 (Rendering|Material|CreateDynamicMaterialInstance "/Game/BLUCA/M_DrawMaskFade.M_DrawMaskFade" "None" "None" :!class /Script/Engine.KismetMaterialLibrary))
      (Variables|Default|SetFadeMaterial _returnvalue_3)
      (Rendering|ClearRenderTarget2D "/Game/BLUCA/RT_DrawMaskFade.RT_DrawMaskFade"))))

(event EventTick
  (params (DeltaSeconds :type Float%20%28single-precision%29))
  (CallFunction|DrawFade (* DeltaSeconds (Variables|Default|GetFadeSpeed)))
  (CallFunction|DrawBuffer)
  (Rendering|ClearRenderTarget2D "/Game/BLUCA/RT_DrawMask.RT_DrawMask"))

(fn ConstructionScript)

(fn PaintActor
  (params (ActorToPaint :type Skeletal%20Mesh%20Actor%20Object%20Reference) (HitLocation :type Vector) (BrushRadius :type Float%20%28single-precision%29))
  (LocalVariables|SetMeshComponent (Variables|/Script/Engine.SkeletalMeshActor|GetSkeletalMeshComponent ActorToPaint))
  (Utilities|FlowControl|Sequence
    (:then_0
      (LocalVariables|SetOriginalMaterial (Rendering|Material|GetMaterial (LocalVariables|GetMeshComponent) 0))
      (Rendering|Material|SetMaterial (LocalVariables|GetMeshComponent) 0 (Variables|Default|GetUnwrapMaterial)))
    (:then_1
      (Rendering|Material|SetVectorParameterValue (Variables|Default|GetUnwrapMaterial) "HitLocation" (Math|Conversions|ToLinearColor(Vector) HitLocation) :!class /Script/Engine.MaterialInstanceDynamic)
      (Rendering|Material|SetScalarParameterValue (Variables|Default|GetUnwrapMaterial) "BrushRadius" 2.0 :!class /Script/Engine.MaterialInstanceDynamic))
    (:then_2
      (Rendering|SceneCapture|CaptureScene (Variables|Default|GetSceneCapture) :!class /Script/Engine.SceneCaptureComponent2D)
      (Rendering|Material|SetMaterial (LocalVariables|GetMeshComponent) 0 (LocalVariables|GetOriginalMaterial)))))

(fn DrawBuffer
  (Rendering|DrawMaterialtoRenderTarget "/Game/BLUCA/RT_DrawMaskBuffer.RT_DrawMaskBuffer" (Variables|Default|GetBufferMaterial)))

(fn DrawFade
  (params (FadeSpeed :type Float%20%28single-precision%29))
  (Rendering|Material|SetScalarParameterValue "/Game/BLUCA/MPC_Global.MPC_Global" "FadeSpeed" FadeSpeed :!class /Script/Engine.KismetMaterialLibrary)
  (Rendering|DrawMaterialtoRenderTarget "/Game/BLUCA/RT_DrawMaskFade.RT_DrawMaskFade" (Variables|Default|GetFadeMaterial)))